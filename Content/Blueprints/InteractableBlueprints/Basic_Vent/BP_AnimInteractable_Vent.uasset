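; Animated interactable vent that characters open or close from inside or outside, enter and exit.
; A vent enum maps interaction IDs to character and object animation maps for each action.
; After each interactor is chosen, it enables either the opened or closed interactor set, starting with the opened set on BeginPlay.
; When an enter or exit animation starts, it notifies the interacting character.
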(event EventBeginPlay
  (Utilities|RevealOpenedInteractors))

(event Collision|EventActorBeginOverlap
  (params (OtherActor :type Actor%20Object%20Reference)))

(event EventTick
  (params (DeltaSeconds :type Float%20%28single-precision%29)))

(event EventOnRequestedAnimStarted
  (switch Utilities|FlowControl|Switch|SwitchonVentEnumerator (Utilities|Enum|ByteToEnumVentEnumerator (Variables|Default|GetCurrent%20Interaction%20ID))
    (:NewEnumerator3
      (Class|VentUserInterface|OnStartEnterVent(Message) (Variables|Default|GetInteracting%20Character)))
    (:NewEnumerator5
      (Class|VentUserInterface|OnStartExitVent(Message) (Variables|Default|GetInteracting%20Character)))))

(fn ConstructionScript
  (|CallParentFunction))

(fn GetCorrectAnimMaps
  (params (In%20Interaction :type Byte :default 0) (In%20Interaction%20User%20Type :type InteractionUserType%20Enum :default "Undefined"))
  (bind _returnvalue (Utilities|Enum|ByteToEnumVentEnumerator In%20Interaction))
  (bind _dooropenfrominside (Variables|Default|GetDoorOpenFromInside))
  (bind _dooropenfromoutside (Variables|Default|GetDoorOpenFromOutside))
  (bind _doorclosefrominside (Variables|Default|GetDoorCloseFromInside))
  (bind _doorclosefromoutside (Variables|Default|GetDoorCloseFromOutside))
  (bind _enter (Variables|Default|GetEnter))
  (bind _exit (Variables|Default|GetExit))
  (bind _returnvalue_2 (Utilities|Select :Index _returnvalue :NewEnumerator0 _dooropenfrominside :NewEnumerator4 _dooropenfromoutside :NewEnumerator1 _doorclosefrominside :NewEnumerator2 _doorclosefromoutside :NewEnumerator3 _enter :NewEnumerator5 _exit))
  (bind (_characteranimmap _objectanimmap) (Utilities|Struct|BreakEntityDoubleAnimMap _returnvalue_2))
  (return _characteranimmap _objectanimmap))

(fn ChooseInteractorstoReveal
  (params (Interactor%20Id :type Byte :default 0))
  (|CallParentFunction Interactor%20Id)
  (switch Utilities|FlowControl|Switch|SwitchonVentEnumerator (Utilities|Enum|ByteToEnumVentEnumerator Interactor%20Id)
    (:NewEnumerator0
      (Utilities|RevealOpenedInteractors :!label _label))
    (:NewEnumerator4
      (goto _label))
    (:NewEnumerator1
      (Utilities|RevealClosedInteractors :!label _label_2))
    (:NewEnumerator2
      (goto _label_2))
    (:NewEnumerator3
      (goto _label))
    (:NewEnumerator5
      (goto _label))))