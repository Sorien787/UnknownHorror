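; Interactable valve that a player turns left or right in steps to drive a list of controlled objects.
; Input moves a clamped wheel state and plays enum-keyed paired character and object animations, chained through completion events.
; An anim notify rotates the mesh, then switches the objects on or off at either end, or sends a progress ratio in between.
; Only users whose owner implements ValveAnimInterface can interact.
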(event EventBeginPlay
  (CallFunction|ChooseInteractorstoReveal)
  (Actor|Tick|SetActorTickEnabled false)
  (if (Variables|Setup|GetStartOnline)
    (Variables|Default|SetCurrentWheelState (Variables|Setup|GetEndWheelState))))

(event EventPlayChangedHands
  (CallFunction|CallAnimationUsingID (Utilities|Enum|LiteralenumWheelEnumerator "NewEnumerator4")))

(event EventPlayRotateRight
  (CallFunction|CallAnimationUsingID (Utilities|Enum|LiteralenumWheelEnumerator "NewEnumerator2"))
  (Variables|Default|SetCurrentWheelAng (+ (Variables|Setup|GetWheelAngChange) (Variables|Default|GetCurrentWheelAng)))
  (Audio|PlaySoundatLocation (select (Utilities|IsatEnd) (Variables|Default|GetFinishRotateSound) (Variables|Default|GetRotateSound)) (Transformation|GetActorLocation) "0, 0, 0" 1.0 1.0 0.0 0 0 0))

(event EventPlayRotateLeft
  (CallFunction|CallAnimationUsingID (Utilities|Enum|LiteralenumWheelEnumerator "NewEnumerator1"))
  (Variables|Default|SetCurrentWheelAng (- (Variables|Default|GetCurrentWheelAng) (Variables|Setup|GetWheelAngChange)))
  (Audio|PlaySoundatLocation (select (Utilities|IsatEnd) (Variables|Default|GetFinishRotateSound) (Variables|Default|GetRotateSound)) (Transformation|GetActorLocation) "0, 0, 0" 1.0 1.0 0.0 0 0 0))

(event EventPlayEnterAnim
  (CallFunction|CallAnimationUsingID (Utilities|Enum|LiteralenumWheelEnumerator "NewEnumerator0")))

(event EventOnAnimationinCompleted
  (Variables|Default|SetNumWaitingAnims 0)
  (CallFunction|PlayEnterAnim))

(event EventOnAnimNotify
  (params (NotifyName :type Name :default "None"))
  (switch name NotifyName
    (:OnValveTurned
      (Transformation|SetRelativeRotation (Variables|Default|GetObjectSkeletalMesh) (Class|KismetMathLibrary|QuatRotator (Class|KismetMathLibrary|QuatMakefromEuler (Math|Vector|MakeVector (Variables|Default|GetCurrentWheelAng) 9e+01 0.0))) false false)
      (if (Utilities|IsatEnd)
        (if (== (Variables|Setup|GetEndWheelState) (Variables|Default|GetCurrentWheelState))
          (for _array_element (Variables|Setup|GetControlled%20Objects)
            (Default|OnSwitchon _array_element))
          (else
            (for _array_element_2 (Variables|Setup|GetControlled%20Objects)
              (Default|OnSwitchOff _array_element_2))))
        (else
          (for _array_element_3 (Variables|Setup|GetControlled%20Objects)
            (Default|OnChangeState _array_element_3 (/ (Math|Conversions|ToFloat(Integer) (Variables|Default|GetCurrentWheelState)) (Math|Conversions|ToFloat(Integer) (Variables|Setup|GetEndWheelState))))))))))

(event EventPlayIdleAnim
  (CallFunction|CallAnimationUsingID (Utilities|Enum|LiteralenumWheelEnumerator "NewEnumerator9"))
  (Variables|Default|SetNumWaitingAnims 0))

(event EventOnRequestedAnimsComplete
  (switch Utilities|FlowControl|Switch|SwitchonWheelEnumerator (Utilities|Enum|ByteToEnumWheelEnumerator (Variables|Default|GetCurrent%20Interaction%20ID))
    (:NewEnumerator0
      (CallFunction|PlayIdleAnim))
    (:NewEnumerator3
      (CallFunction|OnInteractionStopped))
    (:NewEnumerator1
      (if (Utilities|IsatEnd) :!label _label
        (CallFunction|PlayExitAnim)
        (else
          (CallFunction|PlayChangedHands))))
    (:NewEnumerator2
      (goto _label))
    (:NewEnumerator4
      (CallFunction|PlayIdleAnim))))

(event EventPlayExitAnim
  (CallFunction|CallAnimationUsingID (Utilities|Enum|LiteralenumWheelEnumerator "NewEnumerator3")))

(event Input|ActionEvents|InputActionInteract
  (params (Key :type Key%20Structure))
  (:Pressed
    (if (CallFunction|CheckAnimAble)
      (CallFunction|PlayExitAnim))))

(event Input|ActionEvents|InputActionWheelTurnLeft
  (params (Key :type Key%20Structure))
  (:Pressed
    (if (CallFunction|CheckAnimAble)
      (if (!= (Variables|Default|GetCurrentWheelState) 0)
        (Math|Integer|DecrementInt (Variables|Default|GetCurrentWheelState)
          (:%20%20
            (CallFunction|PlayRotateLeft)))))))

(event Input|ActionEvents|InputActionWheelTurnRight
  (params (Key :type Key%20Structure))
  (:Pressed
    (if (CallFunction|CheckAnimAble)
      (if (!= (Variables|Setup|GetEndWheelState) (Variables|Default|GetCurrentWheelState))
        (Math|Integer|IncrementInt (Variables|Default|GetCurrentWheelState)
          (:%20%20
            (CallFunction|PlayRotateRight)))))))

(fn ConstructionScript
  (|CallParentFunction))

(fn OnInteractionStarted
  (params (User%20Component :type Interaction%20User%20Component%20Object%20Reference) (Interactor%20Id :type Integer) (Interaction%20Point%20Pos :type Vector :default "0, 0, 0") (Interaction%20Point%20Rot :type Rotator :default "0, 0, 0"))
  (|CallParentFunction User%20Component Interactor%20Id Interaction%20Point%20Pos Interaction%20Point%20Rot)
  (Actor|Tick|SetActorTickEnabled true))

(fn OnInteractionStopped
  (|CallParentFunction)
  (Actor|Tick|SetActorTickEnabled false))

(fn ChooseInteractorstoReveal
  (params (Interactor%20Id :type Byte :default 0))
  (|CallParentFunction 0)
  (Class|InteractableInterface|OnInteractorIdEnabledSet (Math|Conversions|ToInteger(Byte) (Utilities|Enum|LiteralenumWheelEnumerator "NewEnumerator0"))))

(fn GetCorrectAnimMaps
  (params (In%20Interaction :type Byte :default 0) (In%20Interaction%20User%20Type :type InteractionUserType%20Enum :default "Undefined"))
  (bind _returnvalue (Utilities|Enum|ByteToEnumWheelEnumerator In%20Interaction))
  (bind _enteranims (Variables|Anims|GetEnterAnims))
  (bind _turnrightanims (Variables|Anims|GetTurnRightAnims))
  (bind _turnleftanims (Variables|Anims|GetTurnLeftAnims))
  (bind _finishedanims (Variables|Anims|GetFinishedAnims))
  (bind _handchangeanims (Variables|Anims|GetHandChangeAnims))
  (bind _idleanims (Variables|Anims|GetIdleAnims))
  (bind _returnvalue_2 (Utilities|Select :Index _returnvalue :NewEnumerator0 _enteranims :NewEnumerator3 _finishedanims :NewEnumerator1 _turnleftanims :NewEnumerator2 _turnrightanims :NewEnumerator4 _handchangeanims :NewEnumerator9 _idleanims))
  (bind (_characteranimmap _objectanimmap) (Utilities|Struct|BreakEntityDoubleAnimMap _returnvalue_2))
  (return _characteranimmap _objectanimmap))

(fn IsInteractionAvailableOverride
  (params (interactorId :type Integer) (pInteractionUser :type Interaction%20User%20Component%20Object%20Reference))
  (return (Utilities|DoesObjectImplementInterface (Components|GetOwner pInteractionUser) "/Game/Blueprints/InteractableBlueprints/Valve/ValveAnimInterface.ValveAnimInterface_C")))