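; Base Blueprint for interactable objects that handles starting and stopping a character's interaction with the object.
; Interacting records the user type, interactor ID and owning Character, then sends that character a start message with the object type and itself.
; It then disables interactors through ChooseInteractorsToReveal and fires the empty OnSetupFinished event.
; Stopping sends the character a stop message and calls OnAnimationFinished.
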(event Custom|On%20Setup%20Finished)

(fn ConstructionScript)

(fn OnInteractionStarted
  (params (User%20Component :type Interaction%20User%20Component%20Object%20Reference) (Interactor%20Id :type Integer))
  (Variables|Default|SetCurrent%20User (Variables|/Script/DeepSeaHorror.InteractionUserComponent|Getm_UserType User%20Component))
  (Variables|Default|SetCurrent%20Interaction%20ID (Math|Conversions|ToByte(Integer) Interactor%20Id))
  (bind _ascharacter (Utilities|Casting|CastToCharacter (Components|GetOwner User%20Component)))
  (bind _output_get (Variables|Default|SetInteracting%20Character _ascharacter))
  (Class|CharacterAnimInterface|OnStartObjectInteraction(Message) _output_get (Variables|Default|GetObject%20Type) self)
  (return))

(fn OnInteractionStopped
  (Class|CharacterAnimInterface|OnStopObjectInteraction(Message) (Variables|Default|GetInteracting%20Character) self)
  (Class|InteractableInterface|OnAnimationFinished)
  (return))

(fn ChooseInteractorstoReveal
  (params (Interactor%20Id :type Byte))
  (Class|InteractableInterface|DisableInteractors)
  (return))

(fn OnInteractwithInteractorId2
  (params (interactorId :type Integer) (pInteractionUser :type Interaction%20User%20Component%20Object%20Reference))
  (CallFunction|OnInteractionStarted pInteractionUser interactorId)
  (CallFunction|ChooseInteractorstoReveal (Math|Conversions|ToByte(Integer) interactorId))
  (CallFunction|OnSetupFinished)
  (return true))