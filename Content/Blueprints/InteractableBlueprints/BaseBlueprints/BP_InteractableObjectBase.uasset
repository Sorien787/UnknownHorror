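; BP_InteractableObjectBase is a base Blueprint for objects that characters interact with through interactor points.
; An interaction records the user type and interactor ID, messages the user's Character with the object and its type, disables interactors and calls the empty OnSetupFinished event.
; Stopping messages that Character again and calls OnAnimationFinished.
; The point position and rotation are passed along but unused here, and interactor selection simply disables interactors.
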(event Custom|On%20Setup%20Finished)

(fn ConstructionScript)

(fn OnInteractionStarted
  (params (User%20Component :type Interaction%20User%20Component%20Object%20Reference) (Interactor%20Id :type Integer) (Interaction%20Point%20Pos :type Vector) (Interaction%20Point%20Rot :type Rotator))
  (Variables|InteractableObjectBase|SetCurrent%20User (Variables|/Script/DeepSeaHorror.InteractionUserComponent|Getm_UserType User%20Component))
  (Variables|InteractableObjectBase|SetCurrent%20Interaction%20ID (Math|Conversions|ToByte(Integer) Interactor%20Id))
  (bind _ascharacter (Utilities|Casting|CastToCharacter (Components|GetOwner User%20Component)))
  (bind _output_get (Variables|InteractableObjectBase|SetInteracting%20Character _ascharacter))
  (Class|CharacterAnimInterface|OnStartObjectInteraction(Message) _output_get (Variables|InteractableObjectBase|GetObject%20Type) self)
  (return))

(fn OnInteractionStopped
  (Class|CharacterAnimInterface|OnStopObjectInteraction(Message) (Variables|InteractableObjectBase|GetInteracting%20Character) self)
  (Class|InteractableInterface|OnAnimationFinished)
  (return))

(fn ChooseInteractorstoReveal
  (params (Interactor%20Id :type Byte))
  (Class|InteractableInterface|DisableInteractors)
  (return))

(fn OnInteractwithInteractorId2
  (params (interactorId :type Integer) (pInteractionUser :type Interaction%20User%20Component%20Object%20Reference) (pointRelativePosition :type Vector :default "0, 0, 0") (pointRelativeRotation :type Quat%20Structure))
  (CallFunction|OnInteractionStarted pInteractionUser interactorId pointRelativePosition (Class|KismetMathLibrary|QuatRotator pointRelativeRotation))
  (CallFunction|ChooseInteractorstoReveal (Math|Conversions|ToByte(Integer) interactorId))
  (CallFunction|OnSetupFinished)
  (return true))