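; Interactable ladder that a character enters at top or bottom and climbs rung by rung through animations.
; The construction script repeats mesh pieces along the EndOfLadder length, sets the rung count and places the bottom interactor.
; MoveForward steps a rung index, picking left or right animations from an alternating side flag and exiting at either end.
; Animation completion returns to idle or ends the interaction, while anim notifies play audio at the character.
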(event Custom|OnClimbUp
  (if (Variables|InternalLogic|GetRightSideLower)
    (CallFunction|CallAnimationUsingID (Utilities|Enum|LiteralenumLadderEnumeration "NewEnumerator9"))
    (else
      (CallFunction|CallAnimationUsingID (Utilities|Enum|LiteralenumLadderEnumeration "NewEnumerator4"))))
  (Variables|InternalLogic|SetRightSideLower (not (Variables|InternalLogic|GetRightSideLower))))

(event Custom|PlayIdle
  (if (Variables|InternalLogic|GetRightSideLower)
    (CallFunction|CallAnimationUsingID (Utilities|Enum|LiteralenumLadderEnumeration "NewEnumerator11"))
    (else
      (CallFunction|CallAnimationUsingID (Utilities|Enum|LiteralenumLadderEnumeration "NewEnumerator8"))))
  (Variables|Default|SetNumWaitingAnims 0))

(event Custom|OnReachBottom
  (if (Variables|InternalLogic|GetRightSideLower)
    (CallFunction|CallAnimationUsingID (Utilities|Enum|LiteralenumLadderEnumeration "NewEnumerator3"))
    (else
      (CallFunction|CallAnimationUsingID (Utilities|Enum|LiteralenumLadderEnumeration "NewEnumerator2")))))

(event Custom|OnClimbDown
  (if (Variables|InternalLogic|GetRightSideLower)
    (CallFunction|CallAnimationUsingID (Utilities|Enum|LiteralenumLadderEnumeration "NewEnumerator10"))
    (else
      (CallFunction|CallAnimationUsingID (Utilities|Enum|LiteralenumLadderEnumeration "NewEnumerator5"))))
  (Variables|InternalLogic|SetRightSideLower (not (Variables|InternalLogic|GetRightSideLower))))

(event Custom|OnReachTop
  (if (Variables|InternalLogic|GetRightSideLower)
    (CallFunction|CallAnimationUsingID (Utilities|Enum|LiteralenumLadderEnumeration "NewEnumerator7"))
    (else
      (CallFunction|CallAnimationUsingID (Utilities|Enum|LiteralenumLadderEnumeration "NewEnumerator6")))))

(event EventBeginPlay
  (CallFunction|ChooseInteractorstoReveal))

(event EventOnAnimNotify
  (params (NotifyName :type Name :default "None"))
  (switch name NotifyName
    (:LadderTouch
      (Transformation|SetWorldLocation (Variables|Default|GetLadderAudio) (Transformation|GetWorldLocation (Variables|/Script/Engine.Character|GetCapsuleComponent (Variables|Default|GetInteracting%20Character))) false false)
      (Audio|Components|Audio|Play (Variables|Default|GetLadderAudio) 0.0))))

(event EventOnRequestedAnimsComplete
  (switch Utilities|FlowControl|Switch|SwitchonLadderEnumeration (Utilities|Enum|ByteToEnumLadderEnumeration (Variables|Default|GetCurrent%20Interaction%20ID))
    (:NewEnumerator0
      (Variables|InternalLogic|SetRightSideLower false)
      (Variables|InternalLogic|SetRungIndex 0)
      (CallFunction|PlayIdle :!label _label))
    (:NewEnumerator1
      (Variables|InternalLogic|SetRightSideLower true)
      (Variables|InternalLogic|SetRungIndex (- (Variables|LadderSetup|GetRungCount) (Variables|InternalLogic|GetCharacterRungHeight)))
      (goto _label))
    (:NewEnumerator2
      (CallFunction|OnInteractionStopped :!label _label_2))
    (:NewEnumerator3
      (goto _label_2))
    (:NewEnumerator6
      (goto _label_2))
    (:NewEnumerator7
      (goto _label_2))
    (:NewEnumerator4
      (goto _label))
    (:NewEnumerator9
      (goto _label))
    (:NewEnumerator5
      (goto _label))
    (:NewEnumerator10
      (goto _label))))

(event Input|AxisEvents|InputAxisMoveForward
  (params (AxisValue :type Float%20%28single-precision%29))
  (if (CallFunction|CheckAnimAble)
    (if (!= AxisValue 0.0)
      (if (> AxisValue 0.0)
        (if (== (- (Variables|LadderSetup|GetRungCount) (Variables|InternalLogic|GetCharacterRungHeight)) (Variables|InternalLogic|GetRungIndex))
          (CallFunction|OnReachTop)
          (else
            (CallFunction|OnClimbUp)
            (Math|Integer|IncrementInt (Variables|InternalLogic|GetRungIndex))))
        (elif (== (Variables|InternalLogic|GetRungIndex) 0)
          (CallFunction|OnReachBottom)
          (else
            (CallFunction|OnClimbDown)
            (Math|Integer|DecrementInt (Variables|InternalLogic|GetRungIndex))))))))

(fn ConstructionScript
  (bind _endofladder (Variables|LadderSetup|GetEndOfLadder))
  (bind _piecesize (Variables|LadderSetup|GetPieceSize))
  (bind _returnvalue (Math|Vector|VectorLength _endofladder))
  (bind _returnvalue_2 (Math|Float|Division(WholeandRemainder) _returnvalue _piecesize))
  (Variables|LadderSetup|SetRungCount _returnvalue_2)
  (Utilities|Array|Clear (Variables|LadderSetup|GetRungs))
  (for _index (range 0 _returnvalue_2)
    (AddComponent|AddStaticMeshComponent false (Math|Transform|MakeTransform (Math|Vector|MakeVector 0.0 0.0 (* (* _index (Variables|LadderSetup|GetPieceSize)) -1.0)) "0,180.000000, 0" (Math|Conversions|ToVector(Float) (Variables|Default|GetScale)))))
  (Transformation|SetRelativeLocation (Variables|Default|GetEnterBottomInteractor) (+ (Math|Vector|MakeVector 0.0 0.0 (Math|Conversions|ToFloat(Integer) (Math|Float|Truncate (* (* _returnvalue_2 (Variables|LadderSetup|GetPieceSize)) -1.0)))) (.Location (Math|Transform|BreakTransform (Transformation|GetRelativeTransform (Variables|Default|GetEnterBottomInteractor))))) false false)
  (|CallParentFunction))

(fn GetCorrectAnimMaps
  (params (In%20Interaction :type Byte :default 0) (In%20Interaction%20User%20Type :type InteractionUserType%20Enum :default "Undefined"))
  (return (Utilities|Select :Index (Utilities|Enum|ByteToEnumLadderEnumeration In%20Interaction) :NewEnumerator0 (Variables|Anims|GetEnterBottom) :NewEnumerator1 (Variables|Anims|GetEnterTop) :NewEnumerator2 (Variables|Anims|GetExitBottomRLeg) :NewEnumerator3 (Variables|Anims|GetExitBottomLLeg) :NewEnumerator6 (Variables|Anims|GetExitTopLHand) :NewEnumerator7 (Variables|Anims|GetExitTopRHand) :NewEnumerator4 (Variables|Anims|GetClimbUpwardL) :NewEnumerator9 (Variables|Anims|GetClimbUpwardR) :NewEnumerator5 (Variables|Anims|GetClimbDownwardR) :NewEnumerator10 (Variables|Anims|GetClimbDownwardL) :NewEnumerator11 (Variables|Anims|GetIdleLAnims) :NewEnumerator8 (Variables|Anims|GetIdleRAnims)) ""))

(fn ChooseInteractorstoReveal
  (params (Interactor%20Id :type Byte :default 0))
  (|CallParentFunction 0)
  (Class|InteractableInterface|OnInteractorIdEnabledSet (Math|Conversions|ToInteger(Byte) (Utilities|Enum|LiteralenumLadderEnumeration "NewEnumerator0")))
  (Class|InteractableInterface|OnInteractorIdEnabledSet (Math|Conversions|ToInteger(Byte) (Utilities|Enum|LiteralenumLadderEnumeration "NewEnumerator1"))))