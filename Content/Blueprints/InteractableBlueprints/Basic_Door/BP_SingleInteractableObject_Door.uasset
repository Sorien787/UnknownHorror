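; Single interactable door that swaps between open and close interactions, each available from the outward and inward side.
; On BeginPlay it enables the two open interactors.
; When choosing interactors to reveal, an open interaction enables both close interactors and a close interaction enables both open ones.
; GetCorrectAnimMaps maps the door enum to the matching character and object animation maps.
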(event EventBeginPlay
  (Utilities|RevealOpenInteractors))

(fn ConstructionScript
  (|CallParentFunction))

(fn GetCorrectAnimMaps
  (params (In%20Interaction :type Byte :default 0) (In%20Interaction%20User%20Type :type InteractionUserType%20Enum :default "Undefined"))
  (bind _returnvalue (Utilities|Enum|ByteToEnumDefaultDoorEnumerator In%20Interaction))
  (bind _dooropenoutwardsmap (Variables|Default|GetDoorOpenOutwardsMap))
  (bind _dooropeninwardsmap (Variables|Default|GetDoorOpenInwardsMap))
  (bind _doorcloseinwardsmap (Variables|Default|GetDoorCloseInwardsMap))
  (bind _doorcloseoutwardsmap (Variables|Default|GetDoorCloseOutwardsMap))
  (bind _returnvalue_2 (Utilities|Select :Index _returnvalue :NewEnumerator0 _dooropenoutwardsmap :NewEnumerator1 _dooropeninwardsmap :NewEnumerator2 _doorcloseoutwardsmap :NewEnumerator3 _doorcloseinwardsmap))
  (bind (_characteranimmap _objectanimmap) (Utilities|Struct|BreakEntityDoubleAnimMap _returnvalue_2))
  (return _characteranimmap _objectanimmap))

(fn ChooseInteractorstoReveal
  (params (Interactor%20Id :type Byte :default 0))
  (|CallParentFunction 0)
  (switch Utilities|FlowControl|Switch|SwitchonDefaultDoorEnumerator (Utilities|Enum|ByteToEnumDefaultDoorEnumerator Interactor%20Id)
    (:NewEnumerator0
      (Utilities|RevealCloseInteractors :!label _label))
    (:NewEnumerator1
      (goto _label))
    (:NewEnumerator2
      (Utilities|RevealOpenInteractors :!label _label_2))
    (:NewEnumerator3
      (goto _label_2))))