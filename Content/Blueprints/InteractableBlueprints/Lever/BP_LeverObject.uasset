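; Lever interactable Blueprint with two interactions, Up and Down, built on a parent interactable class.
; It overrides animation lookup, converting the interaction to a lever enum to return the matching pull-up or pull-down character and object animation maps.
; After the parent's interactor reveal logic runs, it enables the opposite direction's interactor, so Up reveals Down and Down reveals Up.
; The event graph holds no active logic.
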(event EventBeginPlay)

(event Collision|EventActorBeginOverlap
  (params (OtherActor :type Actor%20Object%20Reference)))

(event EventTick
  (params (DeltaSeconds :type Float%20%28single-precision%29)))

(fn ConstructionScript
  (|CallParentFunction))

(fn GetCorrectAnimMaps
  (params (In%20Interaction :type Byte :default 0) (In%20Interaction%20User%20Type :type InteractionUserType%20Enum :default "Undefined"))
  (bind _returnvalue (Utilities|Enum|ByteToEnumLeverEnumeration In%20Interaction))
  (bind _level_pull_up_anim (Variables|Default|GetLevel%20Pull%20Up%20Anim))
  (bind _level_pull_down_anims (Variables|Default|GetLevel%20Pull%20Down%20Anims))
  (bind _returnvalue_2 (Utilities|Select :Index _returnvalue :NewEnumerator0 _level_pull_up_anim :NewEnumerator1 _level_pull_down_anims))
  (bind (_characteranimmap _objectanimmap) (Utilities|Struct|BreakEntityDoubleAnimMap _returnvalue_2))
  (return _characteranimmap _objectanimmap))

(fn ChooseInteractorstoReveal
  (params (Interactor%20Id :type Byte :default 0))
  (|CallParentFunction 0)
  (switch Utilities|FlowControl|Switch|SwitchonLeverEnumeration (Utilities|Enum|ByteToEnumLeverEnumeration Interactor%20Id)
    (:NewEnumerator0
      (Class|InteractableInterface|OnInteractorIdEnabledSet (Math|Conversions|ToInteger(Byte) (Utilities|Enum|LiteralenumLeverEnumeration "NewEnumerator1"))))
    (:NewEnumerator1
      (Class|InteractableInterface|OnInteractorIdEnabledSet (Math|Conversions|ToInteger(Byte) (Utilities|Enum|LiteralenumLeverEnumeration "NewEnumerator0"))))))