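; Interactable complex door that the player can open or close, either through full animations or by grabbing the handle and controlling the swing gradually.
; Interaction IDs, read as an enum when requested animations complete, either end the interaction or set direction, handle side and hand IK.
; MoveForward input scales into a clamped open value that drives the door AnimBP's blend.
; Peeking, Tick logic and threshold transitions are unfinished stubs.
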(event EventBeginPlay
  (bind _ascomplex_door_anim_bp (Utilities|Casting|CastToComplexDoor_AnimBP (Components|SkeletalMesh|GetAnimInstance (Variables|Default|GetObjectSkeletalMesh)))
    (:then
      _)
    (:CastFailed
      _))
  (Variables|Default|SetDoor%20Anim%20BP _ascomplex_door_anim_bp)
  (if (Variables|Default|GetIsOpenByDefault)
    (CallFunction|OpenDoor)
    (else
      (CallFunction|CloseDoor)))
  (|CallParentFunction))

(event Collision|EventActorBeginOverlap
  (params (OtherActor :type Actor%20Object%20Reference))
  (|CallParentFunction OtherActor) ; This node is disabled and will not be called.\nDrag off pins to build functionality.
)

(event EventOnRequestedAnimsComplete
  (switch Utilities|FlowControl|Switch|SwitchonComplexDoorEnumeration (Utilities|Enum|ByteToEnumComplexDoorEnumeration (Variables|Default|GetCurrent%20Interactor%20Id))
    (:NewEnumerator0
      (CallFunction|OnInteractionStopped :!label _label))
    (:NewEnumerator1
      (goto _label))
    (:NewEnumerator2
      (goto _label))
    (:NewEnumerator3
      (goto _label))
    (:NewEnumerator4
      (CallFunction|SetIsOpeningDoor)
      (CallFunction|IsInsideDoor))
    (:NewEnumerator5
      (CallFunction|SetIsOpeningDoor)
      (CallFunction|IsOutsideDoor))
    (:NewEnumerator6
      (CallFunction|SetIsClosingDoor)
      (CallFunction|IsInsideDoor))
    (:NewEnumerator7
      (CallFunction|SetIsClosingDoor)
      (CallFunction|IsOutsideDoor))))

(event EventTick
  (params (DeltaSeconds :type Float%20%28single-precision%29))
  (if (Variables|Default|GetIsInComplexAnim)
    _))

(event Input|AxisEvents|InputAxisMoveForward
  (params (AxisValue :type Float%20%28single-precision%29))
  ;[1 1 1] Try Opening/Closing Door More
  (CallFunction|SetDoorOpenVal (Math|Float|Clamp(Float) (+ (* (Variables|Default|GetDoorSensitivity) (Utilities|Time|GetWorldDeltaSeconds) (Variables|Default|GetDoorStepMultiplier) AxisValue) (Variables|Default|GetCurrentDoorOpenVal))))
  (if (<= (Variables|Default|GetCurrentDoorOpenVal) (Variables|Default|GetDoorReturnTolerance))
    (if (Variables|Default|GetIsOpeningDoor)
      _)
    (elif (> (Variables|Default|GetCurrentDoorOpenVal) (Variables|Default|GetDoorTransitionPoint))
      (if (Variables|Default|GetIsOpeningDoor)
        _))))

(event Input|AxisEvents|InputAxisMoveRight
  (params (AxisValue :type Float%20%28single-precision%29))
  ;[1 1 1] Try Peeking Left/Right
)

(fn ConstructionScript
  (|CallParentFunction))

(fn SetDoorOpenVal
  (params (DoorOpenVal :type Float%20%28single-precision%29))
  (bind _output_get (Variables|Default|SetCurrentDoorOpenVal DoorOpenVal))
  (Variables|/Game/Blueprints/InteractableBlueprints/Complex_Door/ComplexDoor_AnimBP.ComplexDoor_AnimBP_C|SetDoorOpeningBlend (Variables|Default|GetDoor%20Anim%20BP) _output_get))

(fn CloseDoor
  (Variables|/Game/Blueprints/InteractableBlueprints/Complex_Door/ComplexDoor_AnimBP.ComplexDoor_AnimBP_C|SetIsOpen (Variables|Default|GetDoor%20Anim%20BP) false)
  (CallFunction|SetDoorOpenVal 0.0))

(fn OpenDoor
  (Variables|/Game/Blueprints/InteractableBlueprints/Complex_Door/ComplexDoor_AnimBP.ComplexDoor_AnimBP_C|SetIsOpen (Variables|Default|GetDoor%20Anim%20BP) true)
  (CallFunction|SetDoorOpenVal 1.0))

(fn SetPeekPositions
  (params (MainPos :type Scene%20Component%20Object%20Reference) (LeftHeadTarget :type Scene%20Component%20Object%20Reference) (RightHeadTarget :type Scene%20Component%20Object%20Reference))
  (Variables|Default|SetDefaultHeadTarget MainPos)
  (Variables|Default|SetLeftHeadTarget LeftHeadTarget)
  (Variables|Default|SetRightHeadTarget RightHeadTarget))

(fn IsOutsideDoor
  (Variables|Default|SetCurrentHandle (Variables|Default|GetOuter%20Handle))
  (Variables|Default|SetLeftHeadTarget 0)
  (Variables|Default|SetRightHeadTarget 0)
  (Variables|Default|SetDefaultHeadTarget 0)
  (Variables|/Game/Mannequin/Animations/PlayerAnim/ThirdPerson_AnimBP.ThirdPerson_AnimBP_C|SetRightHandIKEnabled (Variables|Default|GetCharacter%20Anim%20BP) true))

(fn IsInsideDoor
  (Variables|Default|SetCurrentHandle (Variables|Default|GetInner%20Handle))
  (Variables|Default|SetLeftHeadTarget 0)
  (Variables|Default|SetRightHeadTarget 0)
  (Variables|Default|SetDefaultHeadTarget 0)
  (Variables|/Game/Mannequin/Animations/PlayerAnim/ThirdPerson_AnimBP.ThirdPerson_AnimBP_C|SetLeftHandIKEnabled (Variables|Default|GetCharacter%20Anim%20BP) false))

(fn SetIsOpeningDoor
  (Variables|Default|SetIsOpeningDoor true)
  (Variables|Default|SetIsInComplexAnim true)
  (Variables|Default|SetDoorStepMultiplier 1.0))

(fn SetIsClosingDoor
  (Variables|Default|SetIsOpeningDoor false)
  (Variables|Default|SetIsInComplexAnim true)
  (Variables|Default|SetDoorStepMultiplier -1.0))

(fn OnInteractionStarted
  (|CallParentFunction)
  (switch Utilities|FlowControl|Switch|SwitchonComplexDoorEnumeration (Utilities|Enum|ByteToEnumComplexDoorEnumeration (Variables|Default|GetCurrent%20Interactor%20Id))
    (:NewEnumerator4
      _)
    (:NewEnumerator5
      _)
    (:NewEnumerator6
      _)
    (:NewEnumerator7
      _))
  (Actor|Tick|SetActorTickEnabled true))

(fn OnInteractionStopped
  (|CallParentFunction)
  (Actor|Tick|SetActorTickEnabled false))