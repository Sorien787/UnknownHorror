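; An animated interactable light that characters turn on and off, starting in the state set by DefaultState.
; Turn-on and turn-off interactions each select their own character and object animation maps.
; The "FlickSwitch" anim notify drives LightModComponent, so the light changes at that point in the animation.
; Interactor IDs map to an On/Off enum, and choosing one reveals the opposite interactor set.
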(event EventBeginPlay
  (if (Variables|Default|GetDefaultState)
    (Class|LightModifierComponent|Switchon (Variables|Default|GetLight%20Mod%20Component) false)
    (Utilities|RevealOffInteractors)
    (else
      (Class|LightModifierComponent|SwitchOff (Variables|Default|GetLight%20Mod%20Component) false)
      (Utilities|RevealonInteractors))))

(event EventOnAnimNotify
  (params (NotifyName :type Name :default "None"))
  (if (Utilities|Name|Equal(Name) "FlickSwitch" NotifyName)
    (switch Utilities|FlowControl|Switch|SwitchonLightEnumeration (Utilities|Enum|ByteToEnumLightEnumeration (Variables|Default|GetCurrent%20Interactor%20Id))
      (:NewEnumerator0
        (Class|LightModifierComponent|Switchon (Variables|Default|GetLight%20Mod%20Component) false))
      (:NewEnumerator1
        (Class|LightModifierComponent|SwitchOff (Variables|Default|GetLight%20Mod%20Component) false)))))

(fn ConstructionScript
  (|CallParentFunction))

(fn ChooseInteractorstoReveal
  (params (Interactor%20Id :type Byte :default 0))
  (|CallParentFunction 0)
  (switch Utilities|FlowControl|Switch|SwitchonLightEnumeration (Utilities|Enum|ByteToEnumLightEnumeration Interactor%20Id)
    (:NewEnumerator0
      (Utilities|RevealOffInteractors))
    (:NewEnumerator1
      (Utilities|RevealonInteractors))))

(fn GetCorrectAnimMaps
  (params (In%20Interaction :type Byte :default 0) (In%20Interaction%20User%20Type :type InteractionUserType%20Enum :default "Undefined"))
  (bind _turn_on_animations (Variables|Default|GetTurn%20On%20Animations))
  (bind _turn_off_animations (Variables|Default|GetTurn%20Off%20Animations))
  (bind _returnvalue (Utilities|Select :Index In%20Interaction :Option%200 _turn_on_animations :Option%201 _turn_off_animations))
  (bind (_characteranimmap _objectanimmap) (Utilities|Struct|BreakEntityDoubleAnimMap _returnvalue))
  (return _characteranimmap _objectanimmap))