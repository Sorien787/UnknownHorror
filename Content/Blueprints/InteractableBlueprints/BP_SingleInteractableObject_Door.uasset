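; Door variant of a single interactable object, offering open and close interactions from both the inward and outward sides.
; After an interaction, ChooseInteractorsToReveal enables the opposite pair of interactors: opening reveals both close interactors, and closing reveals both open ones.
; GetCorrectAnimMaps selects the matching character and door animation maps for each of the four door interactions.
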(event EventBeginPlay)

(event Collision|EventActorBeginOverlap
  (params (OtherActor :type Actor%20Object%20Reference)))

(event EventTick
  (params (DeltaSeconds :type Float%20%28single-precision%29)))

(fn ConstructionScript
  (|CallParentFunction))

(fn ChooseInteractorstoReveal
  (params (Interactor%20Id :type Byte :default 0))
  (|CallParentFunction Interactor%20Id)
  (switch Utilities|FlowControl|Switch|SwitchonDefaultDoorEnumerator (Utilities|Enum|ByteToEnumDefaultDoorEnumerator Interactor%20Id)
    (:NewEnumerator0
      (Utilities|RevealCloseInteractors :!label _label
        (:Exec%20Out
          _)))
    (:NewEnumerator1
      (goto _label))
    (:NewEnumerator2
      (Utilities|RevealOpenInteractors :!label _label_2
        (:Exec%20out
          _)))
    (:NewEnumerator3
      (goto _label_2)))
  (return))

(fn GetCorrectAnimMaps
  (params (In%20Interaction :type Byte :default 0))
  (bind _returnvalue (Utilities|Enum|ByteToEnumDefaultDoorEnumerator In%20Interaction))
  (return (Utilities|Select :Index _returnvalue :NewEnumerator0 (Variables|Default|GetDoorOpenOutwardsCharacterMap) :NewEnumerator1 (Variables|Default|GetDoorOpenInwardsCharacterMap) :NewEnumerator2 (Variables|Default|GetDoorCloseOutwardsCharacterMap) :NewEnumerator3 (Variables|Default|GetDoorCloseInwardsCharacterMap)) (Utilities|Select :Index _returnvalue :NewEnumerator0 (Variables|Default|GetDoorOpenOutwardsObjectMap) :NewEnumerator1 (Variables|Default|GetDoorOpenInwardsObjectMap) :NewEnumerator2 (Variables|Default|GetDoorCloseOutwardsObjectMap) :NewEnumerator3 (Variables|Default|GetDoorCloseInwardsObjectMap))))