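; Interactable hiding spot that a character enters, leans within and exits through paired character and object animations.
; Interact input plays a quick or slow enter depending on sprint, and completing any exit animation stops the interaction.
; A hiding-spot enum selects the animation maps, and only the two enter interactors are revealed on top of parent logic.
; Lean inputs pass to the character when animation allows, with FB input driving LR lean and vice versa.
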(event Input|EnhancedActionEvents|EnhancedInputActionInputActionHidingLeanFB
  (params (ActionValue :type Float%20%28double-precision%29) (ElapsedSeconds :type Float%20%28double-precision%29) (TriggeredSeconds :type Float%20%28double-precision%29) (InputAction :type Input%20Action%20Object%20Reference :default "/Game/Blueprints/Character/Player/Input/InputActionHidingLeanFB.InputActionHidingLeanFB"))
  (:Triggered
    (if (CallFunction|CheckAnimAble) :!label _label
      (Class|HidingSpotAnimInterface|SetLeaningLR(Message) (Variables|Default|GetInteracting%20Character) (Math|Conversions|ToInteger(Byte) (Class|KismetMathLibrary|ToInt64(Float) ActionValue)))))
  (:Ongoing
    (goto _label)))

(event Input|EnhancedActionEvents|EnhancedInputActionInputActionHidingLeanLR
  (params (ActionValue :type Float%20%28double-precision%29) (ElapsedSeconds :type Float%20%28double-precision%29) (TriggeredSeconds :type Float%20%28double-precision%29) (InputAction :type Input%20Action%20Object%20Reference :default "/Game/Blueprints/Character/Player/Input/InputActionHidingLeanLR.InputActionHidingLeanLR"))
  (:Triggered
    (if (CallFunction|CheckAnimAble) :!label _label
      (Class|HidingSpotAnimInterface|SetLeaningFB(Message) (Variables|Default|GetInteracting%20Character) (Math|Conversions|ToInteger(Byte) (Class|KismetMathLibrary|ToInt64(Float) ActionValue)))))
  (:Ongoing
    (goto _label)))

(event Input|EnhancedActionEvents|EnhancedInputActionInputActionInteract
  (params (ActionValue :type Boolean) (ElapsedSeconds :type Float%20%28double-precision%29) (TriggeredSeconds :type Float%20%28double-precision%29) (InputAction :type Input%20Action%20Object%20Reference :default "/Game/Blueprints/Character/Player/Input/InputActionInteract.InputActionInteract"))
  (:Triggered
    (if (Input|EnhancedActionValues|GetInputActionSprint) :!label _label
      (CallFunction|CallAnimationUsingID (Utilities|Enum|LiteralenumHidingSpotEnum "NewEnumerator1"))
      (else
        (CallFunction|CallAnimationUsingID (Utilities|Enum|LiteralenumHidingSpotEnum "NewEnumerator0")))))
  (:Completed
    (goto _label)))

(event EventOnRequestedAnimsComplete
  (switch Utilities|FlowControl|Switch|SwitchonHidingSpotEnum (Utilities|Enum|ByteToEnumHidingSpotEnum (Variables|Default|GetCurrent%20Interaction%20ID))
    (:NewEnumerator2
      _)
    (:NewEnumerator3
      _)
    (:NewEnumerator8
      _))
  (CallFunction|OnInteractionStopped))

(fn ConstructionScript
  (|CallParentFunction))

(fn GetCorrectAnimMaps
  (params (In%20Interaction :type Byte :default 0) (In%20Interaction%20User%20Type :type InteractionUserType%20Enum :default "Undefined"))
  (bind _returnvalue (Utilities|Enum|ByteToEnumHidingSpotEnum In%20Interaction))
  (bind _enterquickanimmap (Variables|Animation|GetEnterQuickAnimMap))
  (bind _enterslowanimmap (Variables|Animation|GetEnterSlowAnimMap))
  (bind _exitquickanimmap (Variables|Animation|GetExitQuickAnimMap))
  (bind _exitslowanimmap (Variables|Animation|GetExitSlowAnimMap))
  (bind _exitfoundanimmap (Variables|Default|GetExitFoundAnimMap))
  (bind _returnvalue_2 (Utilities|Select :Index _returnvalue :NewEnumerator0 _enterslowanimmap :NewEnumerator1 _enterquickanimmap :NewEnumerator2 _exitslowanimmap :NewEnumerator3 _exitquickanimmap :NewEnumerator8 _exitfoundanimmap))
  (bind (_characteranimmap _objectanimmap) (Utilities|Struct|BreakEntityDoubleAnimMap _returnvalue_2))
  (return _characteranimmap _objectanimmap))

(fn ChooseInteractorstoReveal
  (params (Interactor%20Id :type Byte :default 0))
  (|CallParentFunction Interactor%20Id)
  (Class|InteractableInterface|OnInteractorIdEnabledSet (Math|Conversions|ToInteger(Byte) (Utilities|Enum|LiteralenumHidingSpotEnum "NewEnumerator0")))
  (Class|InteractableInterface|OnInteractorIdEnabledSet (Math|Conversions|ToInteger(Byte) (Utilities|Enum|LiteralenumHidingSpotEnum "NewEnumerator1"))))