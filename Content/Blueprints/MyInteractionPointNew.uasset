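; An interaction point Blueprint that relays interaction state changes to its on-screen prompt widget.
; On BeginPlay it initializes the widget held by the MPInteractWidget component.
; Focus, unfocus, hide, reveal, and fast or slow interact events each forward a matching message to that widget, leaving the visual response to the widget itself.
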(event EventInteractionWidgetFocus
  (Class|InteractableAnimInterface|Focus(Message) (UserInterface|GetWidget (Variables|Default|Getm_pInteractWidget))))

(event EventInteractionWidgetUnfocus
  (Class|InteractableAnimInterface|Unfocus(Message) (UserInterface|GetWidget (Variables|Default|Getm_pInteractWidget))))

(event EventInteractionWidgetReveal
  (Class|InteractableAnimInterface|Reveal(Message) (UserInterface|GetWidget (Variables|Default|Getm_pInteractWidget))))

(event EventInteractionWidgetHide
  (Class|InteractableAnimInterface|Hide(Message) (UserInterface|GetWidget (Variables|Default|Getm_pInteractWidget))))

(event EventInteractionWidgetInteractFast
  (Class|InteractableAnimInterface|Fast(Message) (UserInterface|GetWidget (Variables|Default|Getm_pInteractWidget))))

(event EventInteractionWidgetInteractSlow
  (Class|InteractableAnimInterface|Slow(Message) (UserInterface|GetWidget (Variables|Default|Getm_pInteractWidget))))

(event EventBeginPlay
  (Class|InteractableAnimInterface|Init(Message) (UserInterface|GetWidget (Variables|Default|Getm_pInteractWidget))))

(fn ConstructionScript)