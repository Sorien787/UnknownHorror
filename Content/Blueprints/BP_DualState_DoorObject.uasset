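; A two-state door object Blueprint that responds to three interactor IDs to switch between forward and reverse states.
; Interactor 0 enables interactors 1 and 2 and plays a timeline, while either of those re-enables 0 and reverses it.
; A yaw rotation of DoorMesh scaled from the timeline track is present but unconnected, so this graph never moves the door.
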(event EventOnInteractwithInteractorId
  (params (interactorId :type Integer))
  (switch int interactorId
    (:0
      (Class|InteractableObjectBase|OnInteractorIdEnabledSet 1 true)
      (Class|InteractableObjectBase|OnInteractorIdEnabledSet 2 true)
      (bind _newtrack_0 (Timeline|Timeline_0 Play)))
    (:1
      (Class|InteractableObjectBase|OnInteractorIdEnabledSet 0 true :!label _label)
      (Timeline|Timeline_0 Reverse))
    (:2
      (goto _label))))

(fn ConstructionScript
  (|CallParentFunction))