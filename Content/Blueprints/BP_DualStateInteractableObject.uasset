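; BP_DualStateInteractableObject is an interactable object Blueprint whose visible logic drives an on-screen interaction prompt through its MPInteractWidget component.
; BeginPlay sends an init message to the component's user widget.
; Focus, unfocus, hide, reveal and fast or slow interact events each forward a matching message to that widget.
; The graph holds no dual-state logic, and the construction script is empty.
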(event EventInteractionWidgetFocus
  (Class|InteractableAnimInterface|Focus(Message) (UserInterface|GetUserWidgetObject (Variables|Default|Getm_pInteractWidget))))

(event EventInteractionWidgetInteractFast
  (Class|InteractableAnimInterface|Fast(Message) (UserInterface|GetUserWidgetObject (Variables|Default|Getm_pInteractWidget))))

(event EventInteractionWidgetInteractSlow
  (Class|InteractableAnimInterface|Slow(Message) (UserInterface|GetUserWidgetObject (Variables|Default|Getm_pInteractWidget))))

(event EventBeginPlay
  (Class|InteractableAnimInterface|Init(Message) (UserInterface|GetUserWidgetObject (Variables|Default|Getm_pInteractWidget))))

(event EventInteractionWidgetUnfocus
  (Class|InteractableAnimInterface|Unfocus(Message) (UserInterface|GetUserWidgetObject (Variables|Default|Getm_pInteractWidget))))

(event EventInteractionWidgetHide
  (Class|InteractableAnimInterface|Hide(Message) (UserInterface|GetUserWidgetObject (Variables|Default|Getm_pInteractWidget))))

(event EventInteractionWidgetReveal
  (Class|InteractableAnimInterface|Reveal(Message) (UserInterface|GetUserWidgetObject (Variables|Default|Getm_pInteractWidget))))

(fn ConstructionScript)