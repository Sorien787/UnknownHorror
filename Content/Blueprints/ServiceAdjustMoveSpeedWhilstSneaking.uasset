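; Behavior tree service that adjusts an AI pawn's walk speed while sneaking.
; Each AI tick picks a found-player or not-found base speed from the ActorVisible blackboard bool, then scales it by a curve sampled at the pawn's distance to the ActorLocation blackboard vector.
; MaxWalkSpeed on the character movement component eases toward that target with FInterpTo.
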(event EventReceiveTickAI
  (params (OwnerController :type AI%20Controller%20Object%20Reference) (ControlledPawn :type Pawn%20Object%20Reference) (DeltaSeconds :type Float%20%28single-precision%29))
  (bind _returnvalue (Actor|GetComponentbyClass ControlledPawn "/Script/Engine.CharacterMovementComponent"))
  (Variables|/Script/Engine.CharacterMovementComponent|SetMaxWalkSpeed _returnvalue (Math|Interpolation|FInterpTo (Variables|/Script/Engine.CharacterMovementComponent|GetMaxWalkSpeed _returnvalue) (* (Math|Curves|GetFloatValue (Variables|Default|GetAdditional%20Speed%20By%20Distance) (Math|Vector|Distance(Vector) (Class|BTFunctionLibrary|GetBlackboardValueasVector (Variables|Default|GetActor%20Location)) (Transformation|GetActorLocation ControlledPawn))) (select (Class|BTFunctionLibrary|GetBlackboardValueasBool (Variables|Default|GetActor%20Visible)) (Variables|Default|GetSpeedWhenFoundPlayer) (Variables|Default|GetSpeedWhenNotFoundPlayer))) DeltaSeconds (Variables|Default|GetTimeForIncreaseSpeed))))

(event EventTick
  (params (OwnerActor :type Actor%20Object%20Reference) (DeltaSeconds :type Float%20%28single-precision%29)))