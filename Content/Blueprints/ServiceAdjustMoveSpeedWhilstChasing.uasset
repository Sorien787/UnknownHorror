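; Behavior tree service that adjusts an AI pawn's walk speed while chasing, based on its distance to a perceived location.
; Each tick it measures distance to the blackboard PerceptionLocation and samples the AdditionalSpeedByDistance curve.
; The curve value scales a target between minimum and maximum move speeds, and FInterpTo eases MaxWalkSpeed toward it.
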(event EventReceiveTickAI
  (params (OwnerController :type AI%20Controller%20Object%20Reference) (ControlledPawn :type Pawn%20Object%20Reference) (DeltaSeconds :type Float%20%28single-precision%29))
  (bind _returnvalue (Actor|GetComponentbyClass ControlledPawn "/Script/Engine.CharacterMovementComponent"))
  (Variables|/Script/Engine.CharacterMovementComponent|SetMaxWalkSpeed _returnvalue (Math|Interpolation|FInterpTo (Variables|/Script/Engine.CharacterMovementComponent|GetMaxWalkSpeed _returnvalue) (+ (* (Math|Curves|GetFloatValue (Variables|Default|GetAdditionalSpeedByDistance) (Math|Vector|Distance(Vector) (Transformation|GetActorLocation ControlledPawn) (Class|BTFunctionLibrary|GetBlackboardValueasVector (Variables|Default|GetPerceptionLocation)))) (- (Variables|Default|GetMaxMoveSpeed) (Variables|Default|GetMinMoveSpeed))) (Variables|Default|GetMinMoveSpeed)) DeltaSeconds (Variables|Default|GetTimeToUpdateMovespeed))))